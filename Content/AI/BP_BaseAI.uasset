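; Base AI enemy actor that dies when hit by a SafetyFirstProjectile.
; Death notifies the owning BP_SpawnManager of the kill, if the owner is one, then destroys the actor.
; The construction script caches all SafetyFirstPawn actors and takes the first as Target.
; Tick only stores delta time in Dt, and no movement or attack logic is defined here.
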(event `self.ReceiveHit`
  (params (MyComp :type "PrimitiveComponent Object Reference") (Other :type "Actor Object Reference") (OtherComp :type "PrimitiveComponent Object Reference") (bSelfMoved :type Boolean) (HitLocation :type "Vector Structure") (HitNormal :type "Vector Structure") (NormalImpulse :type "Vector Structure") (Hit :type "HitResult Structure (by ref)"))
  (cast `SafetyFirstProjectile` Other)
  (`self.Death`))

(event `self.ReceiveActorBeginOverlap`
  (params (OtherActor :type "Actor Object Reference")))

(event `self.ReceiveTick`
  (params (DeltaSeconds :type "Float (single-precision)"))
  (set `self.dt` DeltaSeconds))

(fn `Death`
  (bind _asbp_spawn_manager (cast `/Game/AI/BP_SpawnManager` (`self.GetOwner`))
    (:`then`
      (`/Game/AI/BP_SpawnManager.AiKilled` _asbp_spawn_manager))
    (:`CastFailed`
      _))
  (`self.K2_DestroyActor`))

(fn `UserConstructionScript`
  (bind _outactors (`GameplayStatics.GetAllActorsOfClass` "/Script/SafetyFirst.SafetyFirstPawn"))
  (bind _output_get (set `self.PlayerPawns` _outactors))
  (if (> (`KismetArrayLibrary.Array_Length` _output_get) 0)
    (set `self.Target` (`|GetArrayItem` _output_get))))