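; Simple follow AI actor that turns toward and moves after a Target actor each Tick while the target is valid.
; It eases yaw toward the target along the shortest path and takes its forward vector as heading.
; Speed lerps toward MaxSpeed scaled by heading-to-target alignment, clamped at zero, before a swept SetActorLocation.
; Both lerps use per-frame alphas without DeltaSeconds, so smoothing depends on frame rate.
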(event `self.ReceiveBeginPlay`
  (`parent.ReceiveBeginPlay`)
  (set `self.CurrentSpeed` (`KismetMathLibrary.GetForwardVector` (`self.K2_GetActorRotation`))))

(event `self.ReceiveTick`
  (params (DeltaSeconds :type "Float (single-precision)"))
  (bind _target (`self.Target`))
  (`parent.ReceiveTick` DeltaSeconds)
  (`/Engine/EditorBlueprintResources/StandardMacros.IsValid` _target
    (:`Is Valid`
      (set `self.TargetDirection` (- (`self.K2_GetActorLocation` _target) (`self.K2_GetActorLocation`)))
      (`self.UpdateDirection`)
      (`self.UpdateSpeed`)
      (`self.K2_SetActorLocation` (+ (`self.K2_GetActorLocation`) (* (`self.CurrentSpeed`) DeltaSeconds)) true))))

(fn `UpdateDirection`
  (bind (_returnvalue_roll _returnvalue_pitch _returnvalue_yaw) (`KismetMathLibrary.BreakRotator` (`self.K2_GetActorRotation`)))
  (bind (_returnvalue_roll_2 _returnvalue_pitch_2 _returnvalue_yaw_2) (`KismetMathLibrary.BreakRotator` (`KismetMathLibrary.FindLookAtRotation` (`self.K2_GetActorLocation`) (`self.K2_GetActorLocation` (`self.Target`)))))
  (bind (_returnvalue_roll_3 _returnvalue_pitch_3 _returnvalue_yaw_3) (`KismetMathLibrary.BreakRotator` (`KismetMathLibrary.RLerp` (`KismetMathLibrary.MakeRotator` 0.0 0.0 _returnvalue_yaw) (`KismetMathLibrary.MakeRotator` 0.0 0.0 _returnvalue_yaw_2) (`self.RotRelativeLerp`) true)))
  (`self.K2_SetActorRotation` (`KismetMathLibrary.MakeRotator` 0.0 0.0 _returnvalue_yaw_3))
  (set `self.CurrentSpeed` (`SceneComponent.GetForwardVector` (`self.DefaultSceneRoot`))))

(fn `UpdateSpeed`
  (bind _output_get (set `self.fCurrentSpeed` (`KismetMathLibrary.Lerp` (`self.fCurrentSpeed`) (`KismetMathLibrary.FMax` (* (`KismetMathLibrary.Dot_VectorVector` (`self.CurrentSpeed`) (`KismetMathLibrary.Normal` (`self.TargetDirection`))) (`self.MaxSpeed`))) (`self.SpeedRelativeLerp`))))
  (set `self.CurrentSpeed` (* (`KismetMathLibrary.Normal` (`self.CurrentSpeed`)) _output_get)))

(fn `UserConstructionScript`
  (`parent.UserConstructionScript`))