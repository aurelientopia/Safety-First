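; BP_SpawnManager keeps the AI population topped up to MaxAI by spawning through the BP_AISpawner actors in the level.
; It gathers the spawners on BeginPlay and enables spawning after a short delay.
; Tick queues one SpawnAI timer at a time, which picks a random spawner and passes it the manager.
; AiKilled decrements the live count, freeing a slot for another spawn.
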(event `self.ReceiveBeginPlay`
  (bind _outactors (`GameplayStatics.GetAllActorsOfClass` "/Game/AI/BP_AISpawner.BP_AISpawner_C"))
  (set `self.Spawners` _outactors)
  (`KismetSystemLibrary.Delay` 2.0)
  (set `self.CanSpawn` true))

(event `self.ReceiveTick`
  (params (DeltaSeconds :type "Float (single-precision)"))
  (if (and (< (`self.SpawnedAI`) (`self.MaxAI`)) (`self.CanSpawn`) (not (`self.RequestSpawn`)))
    (set `self.RequestSpawn` true)
    (`KismetSystemLibrary.K2_SetTimer` null "SpawnAI" (`self.SpawnDelay`))))

(fn `AiKilled`
  (`/Engine/EditorBlueprintResources/StandardMacros.DecrementInt` (`self.SpawnedAI`)))

(fn `SpawnAI`
  (bind _spawners (`self.Spawners`))
  (`/Game/AI/BP_AISpawner.Spawn` (`|GetArrayItem` _spawners (`KismetMathLibrary.RandomInteger` (`KismetArrayLibrary.Array_Length` _spawners))) self)
  (`/Engine/EditorBlueprintResources/StandardMacros.IncrementInt` (`self.SpawnedAI`)
    (:`  `
      (set `self.RequestSpawn` false))))

(fn `SpawnCooldown`
  (set `self.CanSpawn` true))

(fn `UserConstructionScript`)